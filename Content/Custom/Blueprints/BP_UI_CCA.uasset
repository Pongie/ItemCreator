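; Actor behind the item customization UI that spawns and drives a BP_Item_Actor preview.
; On BeginPlay it spawns the preview from the first DataTable_ItemVisuals row and binds to the GameInstance load callback, which copies TempItemProps.
; CCA2ActorUpdateVisComponents feeds UI values through UpdateItemVariables, remapping offset and rotation and resolving mesh, effect and material by row index, then updates the preview.
; UpdateItemMeshActor applies passed-in item visuals, spawning an actor if none is valid.
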(event `self.ReceiveBeginPlay`
  ;[0 1 0.2331] Init
  (`self.Init`)
  (add `/Game/Custom/Blueprints/BP_GameInstance.GameInstanceLoaded` (`self.As BP Game Instance`) (delegate `GameInstanceLoaded_Event`)))

(event `GameInstanceLoaded_Event`
  (bind _as_bp_game_instance (`self.As BP Game Instance`))
  (set `self.Item Properties Struct` (`/Game/Custom/Blueprints/BP_GameInstance.TempItemProps` _as_bp_game_instance))
  (`KismetSystemLibrary.PrintString` (`.Name_9_545C9A4C441F92FE1DF78391552FF88D` (break `/Game/Custom/Blueprints/Structs/Struct_ItemVisuals` (`.VisualProperties_37_2D6D0A094D0C9C1DAB235EA638DDF488` (break `/Game/Custom/Blueprints/Structs/Struct_ItemProperties` (`|GetArrayItem` (`/Game/Custom/Blueprints/BP_SaveGame.CustomItemsData` (`/Game/Custom/Blueprints/BP_GameInstance.SavedGame` _as_bp_game_instance)))))))))

(fn `CCA2ActorUpdateVisComponents`
  (params (Scale :type "Float (double-precision)") (Offset :type "Float (double-precision)") (Rotation :type "Float (double-precision)") (Mesh :type Integer) (Effect :type Integer) (Mat :type Integer) (Particle :type Boolean))
  (`self.UpdateItemVariables` Scale Offset Rotation Mesh Effect Mat)
  (`/Game/Custom/Blueprints/BP_Item_Actor.UpdateVisualComps` (`self.CurrentItemActor`) Scale (`self.ItemVector`) (`self.ItemRotation`) (`self.Mesh`) (`self.Mat`) (select `bool` Particle :`false` (make `BasicParticleData`) :`true` (make `BasicParticleData`))))

(fn `Init`
  (set `self.As BP Game Instance` (cast `/Game/Custom/Blueprints/BP_GameInstance` (`GameplayStatics.GetGameInstance`) :!pure true))
  (`self.UpdateItemVariables` 0.5 0.5 0.5 0 -1 0) ; Initial load 1 particle 1 material (because datatable is all same mat), and initial mesh
  ;[1 1 1] Load Initial Rotation, Offset, Scale Data from Table
  (bind _outrownames (`DataTableFunctionLibrary.GetDataTableRowNames` "/Game/Custom/Blueprints/DataTables/DataTable_ItemVisuals.DataTable_ItemVisuals"))
  (bind _returnvalue (`|GetDataTableRow` "/Game/Custom/Blueprints/DataTables/DataTable_ItemVisuals.DataTable_ItemVisuals" (`|GetArrayItem` _outrownames))
    (:`then`
      (bind (_name _mesh _material _effect _image _scale _locationoffset _rotationoffset) (break `/Game/Custom/Blueprints/Structs/Struct_ItemVisuals` _returnvalue))
      (bind _returnvalue_2 (`|SpawnActorFromClass` "/Game/Custom/Blueprints/BP_Item_Actor.BP_Item_Actor_C" (`SceneComponent.K2_GetComponentToWorld` (`self.DefaultSceneRoot`)) "Undefined" "OverrideRootScale" null (`self.Item Properties Struct`) (`self.Mesh`) (`self.Emitter Name`) (`self.Particle`) (`self.Material Data`) "Bow" (/ _scale 2.0) _locationoffset _rotationoffset null)) ; Default Vals
      (set `self.CurrentItemActor` _returnvalue_2))))

(fn `Update Item Mesh Actor`
  (params (`Item Properties Struct` :type "/Game/Custom/Blueprints/Structs/Struct_ItemProperties Structure") (Index :type Integer))
  (locals (LocalItemStruct :type "/Game/Custom/Blueprints/Structs/Struct_ItemProperties Structure"))
  (bind ((`VisualProperties_37_2D6D0A094D0C9C1DAB235EA638DDF488` _visualproperties)) (break `/Game/Custom/Blueprints/Structs/Struct_ItemProperties` `Item Properties Struct`))
  (bind _currentitemactor (`self.CurrentItemActor`))
  (bind _currentitemactor_2 (`self.CurrentItemActor`))
  (bind _currentitemactor_3 (`self.CurrentItemActor`))
  (if (!= (`.Name_9_545C9A4C441F92FE1DF78391552FF88D` (break `/Game/Custom/Blueprints/Structs/Struct_ItemVisuals` _visualproperties)) "")
    (bind _structout (setmembers `/Game/Custom/Blueprints/Structs/Struct_ItemProperties` :`StructRef` (make `/Game/Custom/Blueprints/Structs/Struct_ItemProperties` :`VisualProperties` _visualproperties))) ; Update only visual properties from func input parameter
    (`/Engine/EditorBlueprintResources/StandardMacros.IsValid` _currentitemactor_3
      (:`Is Valid`
        (bind _output_get (set `/Game/Custom/Blueprints/BP_Item_Actor.Item Properties Struct` _structout _currentitemactor_3))
        (`/Game/Custom/Blueprints/BP_Item_Actor.UpdateVisualComponentsInitally` _currentitemactor (`.VisualProperties_37_2D6D0A094D0C9C1DAB235EA638DDF488` (break `/Game/Custom/Blueprints/Structs/Struct_ItemProperties` (`/Game/Custom/Blueprints/BP_Item_Actor.Item Properties Struct` _currentitemactor)))))
      (:`Is Not Valid`
        (bind (_name _mesh _material _effect _image _scale) (break `/Game/Custom/Blueprints/Structs/Struct_ItemVisuals` (`.VisualProperties_37_2D6D0A094D0C9C1DAB235EA638DDF488` (break `/Game/Custom/Blueprints/Structs/Struct_ItemProperties` _output_get))))
        (bind _returnvalue (`|SpawnActorFromClass` "/Game/Custom/Blueprints/BP_Item_Actor.BP_Item_Actor_C" (`SceneComponent.K2_GetComponentToWorld` (`self.DefaultSceneRoot`)) "Undefined" "OverrideRootScale" null (`self.Item Properties Struct`) (`self.Mesh`) (`self.Emitter Name`) (`self.Particle`) (`self.Mat`) _name (`KismetMathLibrary.SelectFloat` 1.0 _scale (< _scale 0.5)) (0.0 0.0 0.0) (struct) null :!label _label))
        (set `self.CurrentItemActor` _returnvalue)))
    (else
      (`/Engine/EditorBlueprintResources/StandardMacros.IsValid` _currentitemactor_2
        (:`Is Valid`
          (setmembers `/Game/Custom/Blueprints/Structs/Struct_ItemProperties` :`StructRef` (make `/Game/Custom/Blueprints/Structs/Struct_ItemProperties` :`VisualProperties` _visualproperties)) ; Update only visual properties from func input parameter
          (`/Game/Custom/Blueprints/BP_Item_Actor.UpdateVisualComponentsInitally` _currentitemactor_2 (`.VisualProperties_37_2D6D0A094D0C9C1DAB235EA638DDF488` (break `/Game/Custom/Blueprints/Structs/Struct_ItemProperties` (`|GetArrayItem` (`self.Item Properties Structs`) Index)))))
        (:`Is Not Valid`
          (goto _label))))))

(fn `UpdateItemVariables`
  (params (Scale :type "Float (double-precision)" :default -1.0) (Offset :type "Float (double-precision)" :default -1.0) (Rotation :type "Float (double-precision)" :default -1.0) (Mesh :type Integer :default -1) (Effect :type Integer :default -1) (Mat :type Integer :default -1))
  (bind _returnvalue (`KismetMathLibrary.MakeRotator` (`KismetMathLibrary.MapRangeClamped` Rotation 0.0 1.0 -90.0 90.0)))
  (bind _returnvalue_2 (`KismetMathLibrary.MakeVector` 0.0 0.0 (`KismetMathLibrary.MapRangeClamped` Offset 0.0 1.0 -90.0 90.0)))
  (if (> Scale 0.0)
    (bind _structout (setmembers `/Game/Custom/Blueprints/Structs/Struct_ItemVisuals` :`StructRef` (make `/Game/Custom/Blueprints/Structs/Struct_ItemVisuals` :`Scale` Scale)))
    (setmembers `/Game/Custom/Blueprints/Structs/Struct_ItemProperties` :`StructRef` (make `/Game/Custom/Blueprints/Structs/Struct_ItemProperties` _structout)))
  (if (> Offset 0.0)
    (set `self.ItemVector` _returnvalue_2)
    (bind _structout_2 (setmembers `/Game/Custom/Blueprints/Structs/Struct_ItemVisuals` :`StructRef` (make `/Game/Custom/Blueprints/Structs/Struct_ItemVisuals` :`LocationOffset` _returnvalue_2)))
    (setmembers `/Game/Custom/Blueprints/Structs/Struct_ItemProperties` :`StructRef` (make `/Game/Custom/Blueprints/Structs/Struct_ItemProperties` :`VisualProperties` _structout_2)))
  (if (> Rotation 0.0)
    (set `self.ItemRotation` _returnvalue)
    (bind _structout_3 (setmembers `/Game/Custom/Blueprints/Structs/Struct_ItemVisuals` :`StructRef` (make `/Game/Custom/Blueprints/Structs/Struct_ItemVisuals` :`RotationOffset` _returnvalue)))
    (setmembers `/Game/Custom/Blueprints/Structs/Struct_ItemProperties` :`StructRef` (make `/Game/Custom/Blueprints/Structs/Struct_ItemProperties` :`VisualProperties` _structout_3)))
  (if (> Mesh -1)
    (bind _output_get (set `self.MeshIndex` Mesh))
    (bind _outrownames (`DataTableFunctionLibrary.GetDataTableRowNames` "/Game/Custom/Blueprints/DataTables/DataTable_ItemVisuals.DataTable_ItemVisuals"))
    (bind _returnvalue_3 (`|GetDataTableRow` "/Game/Custom/Blueprints/DataTables/DataTable_ItemVisuals.DataTable_ItemVisuals" (`|GetArrayItem` _outrownames _output_get))
      (:`then`
        (bind ((`Mesh_29_1D6F243B449269BA4433748F57A8B167` _mesh)) (break `/Game/Custom/Blueprints/Structs/Struct_ItemVisuals` _returnvalue_3))
        (set `self.Mesh` _mesh)
        (bind _structout_4 (setmembers `/Game/Custom/Blueprints/Structs/Struct_ItemVisuals` :`StructRef` (make `/Game/Custom/Blueprints/Structs/Struct_ItemVisuals` :`Mesh` _mesh)))
        (setmembers `/Game/Custom/Blueprints/Structs/Struct_ItemProperties` :`StructRef` (make `/Game/Custom/Blueprints/Structs/Struct_ItemProperties` :`VisualProperties` _structout_4)))
      (:`RowNotFound`
        _)))
  (if (> Effect -1)
    (bind _output_get_2 (set `self.EffectIndex` Effect))
    (bind _outrownames_2 (`DataTableFunctionLibrary.GetDataTableRowNames` "/Game/Custom/Blueprints/DataTables/DataTable_ItemVisuals.DataTable_ItemVisuals"))
    (bind _returnvalue_4 (`|GetDataTableRow` "/Game/Custom/Blueprints/DataTables/DataTable_ItemVisuals.DataTable_ItemVisuals" (`|GetArrayItem` _outrownames_2 _output_get_2))
      (:`then`
        (bind _structout_5 (setmembers `/Game/Custom/Blueprints/Structs/Struct_ItemVisuals` :`StructRef` (make `/Game/Custom/Blueprints/Structs/Struct_ItemVisuals` :`Effect` (`.Effect_28_91E2438342AE1E52219207B657B4682B` (break `/Game/Custom/Blueprints/Structs/Struct_ItemVisuals` _returnvalue_4)))))
        (setmembers `/Game/Custom/Blueprints/Structs/Struct_ItemProperties` :`StructRef` (make `/Game/Custom/Blueprints/Structs/Struct_ItemProperties` :`VisualProperties` _structout_5)))
      (:`RowNotFound`
        _)))
  (if (> Mat -1)
    (bind _output_get_3 (set `self.MatIndex` Mat))
    (bind _outrownames_3 (`DataTableFunctionLibrary.GetDataTableRowNames` "/Game/Custom/Blueprints/DataTables/DataTable_ItemVisuals.DataTable_ItemVisuals"))
    (bind _returnvalue_5 (`|GetDataTableRow` "/Game/Custom/Blueprints/DataTables/DataTable_ItemVisuals.DataTable_ItemVisuals" (`|GetArrayItem` _outrownames_3 _output_get_3))
      (:`then`
        (bind _returnvalue_6 (select `int` _output_get_3 :`0` (`.Material_26_7BFA4B9845B040B8ED4D38BB66FAA5BB` (break `/Game/Custom/Blueprints/Structs/Struct_ItemVisuals` _returnvalue_5)) :`1` "/Game/StarterContent/Materials/M_Metal_Gold.M_Metal_Gold" :`2` "/Game/AlchemistsHouse/Assets/Materials/Floor_wooden_texture_Mat.Floor_wooden_texture_Mat"))
        (bind _returnvalue_7 (`KismetMaterialLibrary.CreateDynamicMaterialInstance` _returnvalue_6))
        (set `self.Mat` _returnvalue_7)
        (bind _structout_6 (setmembers `/Game/Custom/Blueprints/Structs/Struct_ItemVisuals` :`StructRef` (make `/Game/Custom/Blueprints/Structs/Struct_ItemVisuals` :`Material` _returnvalue_6)))
        (setmembers `/Game/Custom/Blueprints/Structs/Struct_ItemProperties` :`StructRef` (make `/Game/Custom/Blueprints/Structs/Struct_ItemProperties` :`VisualProperties` _structout_6))))))

(fn `UserConstructionScript`)