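; Item actor whose mesh, material, particle effect and transform are set from visual data, at construction, on BeginPlay and on demand.
; UpdateVisualComponentsInitally applies a visuals struct through a dynamic material instance and clamped scale.
; UpdateVisualComps dispatches changes to per-component updaters, checking material separately and the rest in an else chain.
; UpdateScale multiplies current actor scale by a remapped value, so it compounds; table-data and save hooks are empty.
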(event `self.ReceiveBeginPlay`
  (`self.InitUpdate`))

(event `/Game/Custom/Blueprints/Interface_DataActor.GetTableData`)

(fn `InitUpdate`
  (`self.UpdateMesh`)
  (`self.UpdateParticle`)
  (`self.UpdateMat`)
  (`self.UpdatePosition`)
  (`self.UpdateScale`)
  (`self.UpdateRotation`))

(fn `SaveItemVariables`)

(fn `UpdateMat`
  (bind _materialdata (`self.MaterialData`))
  ;[1 1 1] Mat
  (`/Engine/EditorBlueprintResources/StandardMacros.IsValid` _materialdata
    (:`Is Valid`
      (`PrimitiveComponent.SetMaterial` (`self.StaticMesh`) 0 _materialdata))))

(fn `UpdateMesh`
  (`/Engine/EditorBlueprintResources/StandardMacros.IsValid` (`self.Mesh`)
    (:`Is Valid`
      (`StaticMeshComponent.SetStaticMesh` (`self.StaticMesh`) (`self.Mesh`)))))

(fn `UpdateParticle`
  (bind _particlesys (`self.ParticleSys`))
  (bind _particlesystem (`self.ParticleSystem`))
  ;[1 1 1] Particle
  (`/Engine/EditorBlueprintResources/StandardMacros.IsValid` _particlesys
    (:`Is Valid`
      (`ParticleSystemComponent.SetTemplate` _particlesystem _particlesys)
      (`FXSystemComponent.SetEmitterEnable` _particlesystem (`self.EmitterName`) true))
    (:`Is Not Valid`)))

(fn `UpdatePosition`
  (`self.K2_SetActorRelativeLocation` (`self.Pos`)))

(fn `UpdateRotation`
  (`SceneComponent.K2_SetRelativeRotation` (`self.StaticMesh`) (`self.Rot`) false false))

(fn `UpdateScale`
  (bind _returnvalue (* (`KismetMathLibrary.MapRangeClamped` (`self.Scale`) 50.0 150.0 0.5 1.5) (`self.GetActorScale3D`)))
  (`self.SetActorScale3D` _returnvalue)
  (`KismetSystemLibrary.PrintString` (`KismetStringLibrary.Conv_VectorToString` _returnvalue)))

(fn `UpdateVisualComponentsInitally`
  (params (Visuals :type "/Game/Custom/Blueprints/Structs/Struct_ItemVisuals Structure"))
  (bind (_name _mesh _material _effect _image _scale) (break `/Game/Custom/Blueprints/Structs/Struct_ItemVisuals` Visuals))
  (bind _particlesys (`self.ParticleSys`))
  (bind _materialdata (`self.MaterialData`))
  (bind _staticmesh (`self.StaticMesh`))
  (bind _particlesystem (`self.ParticleSystem`))
  (set `self.Mesh` _mesh)
  (bind _returnvalue (`KismetMaterialLibrary.CreateDynamicMaterialInstance` _material))
  (set `self.MaterialData` _returnvalue)
  (set `self.Particle` _effect)
  (`/Engine/EditorBlueprintResources/StandardMacros.IsValid` (`self.Mesh`)
    (:`Is Valid`
      (`StaticMeshComponent.SetStaticMesh` (`self.StaticMesh`) (`self.Mesh`)))
    (:`Is Not Valid`
      _))
  (`/Engine/EditorBlueprintResources/StandardMacros.IsValid` _particlesys
    (:`Is Valid`
      (`ParticleSystemComponent.SetTemplate` _particlesystem _particlesys)
      (`FXSystemComponent.SetEmitterEnable` _particlesystem (`self.EmitterName`) true))
    (:`Is Not Valid`
      _))
  (`/Engine/EditorBlueprintResources/StandardMacros.IsValid` _materialdata
    (:`Is Valid`
      (`PrimitiveComponent.SetMaterial` _staticmesh 0 _materialdata)
      (`SceneComponent.SetWorldScale3D` _staticmesh (`KismetMathLibrary.ClampVectorSize` (* _scale (`SceneComponent.K2_GetComponentScale` _staticmesh)) 0.5 1.5)))))

(fn `UpdateVisualComps`
  (params (Scale :type "Float (double-precision)") (Pos :type "Vector Structure") (Rot :type "Rotator Structure") (Mesh :type "StaticMesh Object Reference") (Material :type "MaterialInstanceDynamic Object Reference") (Particle :type "BasicParticleData Structure"))
  ;[1 1 1] Since we update 1 component at a time, we dont wanna update everything every time, else we break things
  (if (not (== (`self.MaterialData`) Material))
    (set `self.MaterialData` Material)
    (`self.UpdateMat`))
  (if (not (== (`self.Mesh`) Mesh))
    (set `self.Mesh` Mesh)
    (`self.UpdateMesh`)
    (elif (not (== Scale (`self.Scale`)))
      (set `self.Scale` Scale)
      (`self.UpdateScale`)
      (elif (not (== (`self.Pos`) Pos))
        (set `self.Pos` Pos)
        (`self.UpdatePosition`)
        (elif (not (== (`self.Rot`) Rot))
          (set `self.Rot` Rot)
          (`self.UpdateRotation`)
          (elif (not (== (`.Velocity` (break `BasicParticleData` (`self.Particle`))) (`.Velocity` (break `BasicParticleData` Particle))))
            (set `self.Particle` Particle)
            (`self.UpdateParticle`)))))))

(fn `UserConstructionScript`
  (locals (`Emitter Name` :type Name))
  (bind _particlesys (`self.ParticleSys`))
  (bind _materialdata (`self.MaterialData`))
  (bind _particlesystem (`self.ParticleSystem`))
  (`/Engine/EditorBlueprintResources/StandardMacros.IsValid` (`self.Mesh`)
    (:`Is Valid`
      (`StaticMeshComponent.SetStaticMesh` (`self.StaticMesh`) (`self.Mesh`)))
    (:`Is Not Valid`
      _))
  (`/Engine/EditorBlueprintResources/StandardMacros.IsValid` _particlesys
    (:`Is Valid`
      (`ParticleSystemComponent.SetTemplate` _particlesystem _particlesys)
      (`FXSystemComponent.SetEmitterEnable` _particlesystem (`self.EmitterName`) true))
    (:`Is Not Valid`
      _))
  (`/Engine/EditorBlueprintResources/StandardMacros.IsValid` _materialdata
    (:`Is Valid`
      (`PrimitiveComponent.SetMaterial` (`self.StaticMesh`) 0 _materialdata))))