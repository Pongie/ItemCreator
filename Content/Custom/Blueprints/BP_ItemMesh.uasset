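; BP_ItemMesh is a configurable actor that displays an item as a static mesh with a particle effect.
; The construction script applies the Mesh variable to the StaticMesh component and the Particle template to the ParticleSystem component, each only if valid.
; When a particle template is set, it also enables the emitter named by EmitterName.
; The event graph holds only disabled placeholder events, so the actor runs no gameplay logic.
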(fn `UserConstructionScript`
  (bind _particle (`self.Particle`))
  (bind _particlesystem (`self.ParticleSystem`))
  (`/Engine/EditorBlueprintResources/StandardMacros.IsValid` (`self.Mesh`)
    (:`Is Valid`
      (`StaticMeshComponent.SetStaticMesh` (`self.StaticMesh`) (`self.Mesh`)))
    (:`Is Not Valid`
      _))
  (`/Engine/EditorBlueprintResources/StandardMacros.IsValid` _particle
    (:`Is Valid`
      (`ParticleSystemComponent.SetTemplate` _particlesystem _particle)
      (`FXSystemComponent.SetEmitterEnable` _particlesystem (`self.Emitter Name`) true))))